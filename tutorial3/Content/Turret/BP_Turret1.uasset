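; Turret actor that scans for pawns and fires Ball actors once it locks on.
; Tick spins it while sphere-tracing forward from BarrelL; the first hit becomes a permanent target, which it tracks in yaw and shoots at timed intervals.
; Both BarrelShot branches spawn from BarrelL and clear the flag, so barrels never alternate.
; Closest-visible-target search, smoothed rotation and rate-of-fire functions are unfinished and never called.
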(event EventTick
  (params (DeltaSeconds :type Float%20%28single-precision%29))
  (bind _barrell (Variables|Default|GetBarrelL))
  (bind _barrell_2 (Variables|Default|GetBarrelL))
  (bind _returnvalue (Transformation|GetSocketLocation _barrell "None"))
  (Variables|Components|SetShotTimer (+ (Variables|Components|GetShotTimer) DeltaSeconds))
  (if (Variables|Default|GettargetLocked)
    (Transformation|SetActorRotation (Math|Rotator|MakeRotator 0.0 0.0 (.Yaw (Math|Rotator|BreakRotator (Math|Rotator|FindLookatRotation (Transformation|GetActorLocation) (Transformation|GetActorLocation (Variables|Components|Getplayer)))))))
    (if (> (Variables|Components|GetShotTimer) (Variables|Components|GettimeBetweenShots))
      (Variables|Components|SetShotTimer 0.0)
      (if (Variables|Default|GetBarrelShot)
        (Game|SpawnActorfromClass "/Game/Turret/Ball.Ball_C" (Math|Transform|MakeTransform (Transformation|GetSocketLocation _barrell_2 "None") (Math|Conversions|RotationFromXVector (Transformation|GetActorLocation))) "Undefined" "MultiplyWithRoot" 0 0)
        (Variables|Default|SetBarrelShot false)
        (else
          (Game|SpawnActorfromClass "/Game/Turret/Ball.Ball_C" (Math|Transform|MakeTransform (Transformation|GetSocketLocation _barrell_2 "None") (Transformation|GetActorRotation)) "Undefined" "MultiplyWithRoot" 0 0)
          (Variables|Default|SetBarrelShot false))))
    (else
      (Class|Actor|AddActorWorldRotation (Math|Rotator|MakeRotator 0.0 0.0 (* DeltaSeconds (Variables|Constants|GetRotationSpeed))))
      (bind (_outhit _returnvalue_2) (Collision|SphereTraceForObjects _returnvalue (+ _returnvalue (* (Variables|Components|GetMaxDistance) (Transformation|GetActorForwardVector))) 0.0 (Utilities|Array|MakeArray "ObjectTypeQuery3") false 0 "None"))
      (Variables|Default|SettargetLocked _returnvalue_2)
      (Variables|Components|Setplayer (.HitActor (Collision|BreakHitResult _outhit))))))

(fn ConstructionScript)

(fn FIndBestTarget
  (LocalVariables|SetBestDistance%28Local%29 (stale _result))
  (bind _outactors (Collision|SphereOverlapActors (Transformation|GetActorLocation) 0.0 (Utilities|Array|MakeArray "ObjectTypeQuery3") "/Script/Engine.Actor"))
  (for _array_element _outactors
    (bind _output_get (LocalVariables|SetCurrentTarget%28Local%29 _array_element))
    (bind _output_get_2 (LocalVariables|SetCurrentDistance%28local%29 (Transformation|GetDistanceTo _output_get self)))
    (if (or (< _output_get_2 (LocalVariables|GetBestDistance%28Local%29)) (not (Utilities|IsValid (LocalVariables|GetBestTarget%28Local%29)))) ; Is this the closest?
      (bind _result (CallFunction|HasLineOfSight (Transformation|GetWorldLocation (Variables|Default|GetStaticMeshTop)) (Transformation|GetActorLocation (LocalVariables|GetCurrentTarget%28Local%29)) (Utilities|Array|MakeArray self (LocalVariables|GetCurrentTarget%28Local%29))))
      (if _result
        (LocalVariables|SetBestTarget%28Local%29 (LocalVariables|GetCurrentTarget%28Local%29))
        (LocalVariables|SetBestDistance%28Local%29 (LocalVariables|GetCurrentDistance%28local%29))))))

(fn UpdateTurretRotation
  (params (DeltaSeconds :type Float%20%28double-precision%29)))

(fn UpdateFire
  (if (> (- (Utilities|Time|GetGameTimeinSeconds) 0.0) (Variables|Constants|GetRateOfFire)) ; RateOfFireCooledDown
    _))